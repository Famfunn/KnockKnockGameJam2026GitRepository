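; BP_KitchenCupboardRotate is an interactable kitchen cupboard whose RotatingCupboard mesh swings open temporarily.
; Interact fires the CupboardRotate event and returns that component's static mesh.
; The event snaps the mesh a quarter turn in local space, then reverses it after a short delay, with no interpolation.
; A DoOnce, reset only after the return rotation, blocks repeat triggers mid-cycle.
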(event Custom|CupboardRotate
  (Utilities|FlowControl|DoOnce false :!label _label
    (:Completed
      (Transformation|AddLocalRotation (Variables|Default|GetRotatingCupboard) "0.000000,90.000000,0.000000" false false)
      (Utilities|FlowControl|Delay 5.0)
      (Transformation|AddLocalRotation (Variables|Default|GetRotatingCupboard) "0.000000,-90.000000,0.000000" false false)
      (goto _label Reset))))

(fn ConstructionScript)

(fn Interact
  (CallFunction|CupboardRotate)
  (return (Variables|/Script/Engine.StaticMeshComponent|GetStaticMesh (Variables|Default|GetRotatingCupboard))))