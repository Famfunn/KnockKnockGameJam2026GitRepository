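; BP_SlidingCupboard is an interactable cupboard that shifts sideways and returns by itself after a short delay.
; Interact fires CupboardSlide and returns the SlidingCupboard component's static mesh.
; CupboardSlide moves that component along world Y in an instant, unswept step, then reverses the offset after the delay.
; A DoOnce blocks retriggering until the cupboard is back in place.
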(event Custom|CupboardSlide
  (Utilities|FlowControl|DoOnce false :!label _label
    (:Completed
      (Transformation|AddWorldOffset (Variables|Default|GetSlidingCupboard) "0.000000,52.000000,0.000000" false false)
      (Utilities|FlowControl|Delay 5.0)
      (Transformation|AddWorldOffset (Variables|Default|GetSlidingCupboard) "0.000000,-52.000000,0.000000" false false)
      (goto _label Reset))))

(fn ConstructionScript)

(fn Interact
  (CallFunction|CupboardSlide)
  (return (Variables|/Script/Engine.StaticMeshComponent|GetStaticMesh (Variables|Default|GetSlidingCupboard))))