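; BP_KitchenDrawerTop is an interactable kitchen drawer top whose Door1 component opens on interaction and closes itself five seconds later.
; Interact fires the Door1Open event and returns Door1's static mesh.
; Door1Open snaps the door 90 degrees in local pitch without interpolation, waits, then reverses the rotation.
; A DoOnce blocks re-triggering until the door has closed.
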(event Custom|Door1Open
  ;[1 1 1] On interact, opens the first drawer by rotating it 90 degrees and automatically closes it after 5 seconds
  (Utilities|FlowControl|DoOnce false :!label _label
    (:Completed
      (Transformation|AddLocalRotation (Variables|Default|GetDoor1) (Math|Rotator|MakeRotator 0.0 9e+01 0.0) false false)
      (Utilities|FlowControl|Delay 5.0)
      (Transformation|AddLocalRotation (Variables|Default|GetDoor1) "-90.000000,0.000000,0.000000" false false)
      (goto _label Reset))))

(fn ConstructionScript)

(fn Interact
  (CallFunction|Door1Open)
  (return (Variables|/Script/Engine.StaticMeshComponent|GetStaticMesh (Variables|Default|GetDoor1))))