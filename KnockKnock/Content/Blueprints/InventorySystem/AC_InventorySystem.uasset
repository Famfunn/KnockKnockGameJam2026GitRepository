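; AC_InventorySystem is an inventory component that tracks how many of each item its owner holds.
; A Content map stores a quantity per item, with functions to add, remove and query amounts.
; Add and remove overwrite the entry with the adjusted total; removal clamps at zero and leaves the key in the map.
; The event graph has no active logic.
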(event EventBeginPlay)

(event EventTick
  (params (DeltaSeconds :type Float%20%28single-precision%29)))

(fn AddtoInventory
  (params (Item :type DA%20Item%20Object%20Reference) (Quantity :type Integer))
  (Utilities|Map|Add (Variables|Default|GetContent) Item (+ Quantity (.Value (Utilities|Map|Find (Variables|Default|GetContent) Item)))))

(fn RemovefromInventory
  (params (Item :type DA%20Item%20Object%20Reference) (Quantity :type Integer))
  (Utilities|Map|Add (Variables|Default|GetContent) Item (Math|Integer|Max(Integer) (- (.Value (Utilities|Map|Find (Variables|Default|GetContent) Item)) Quantity))))

(fn QueryInventory
  (params (Item :type DA%20Item%20Object%20Reference))
  (return (.Value (Utilities|Map|Find (Variables|Default|GetContent) Item))))