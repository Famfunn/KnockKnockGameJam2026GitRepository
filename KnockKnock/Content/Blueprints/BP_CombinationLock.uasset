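; BP_CombinationLock is an interactable combination lock that opens a keypad UI when used.
; Interact fires a custom event and returns the object's static mesh.
; The event creates WBP_Keypad, adds it to the viewport, switches player 0 to UI-only input and shows the mouse cursor.
; The Blueprint holds no code-checking or unlock logic.
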(event Custom|CombinationLockEvent
  (bind _returnvalue (Game|GetPlayerController 0))
  (bind _returnvalue_2 (UserInterface|CreateWidget "/Game/UI/WBP_Keypad.WBP_Keypad_C"))
  (UserInterface|Viewport|AddtoViewport _returnvalue_2 0)
  (Input|SetInputModeUIOnly _returnvalue 0 "DoNotLock" false)
  (Variables|/Script/Engine.PlayerController|SetbShowMouseCursor _returnvalue true))

(fn ConstructionScript
  (|CallParentFunction))

(fn Interact
  (CallFunction|CombinationLockEvent)
  (return (Variables|/Script/Engine.StaticMeshComponent|GetStaticMesh (Variables|Default|GetObject%20Mesh))))