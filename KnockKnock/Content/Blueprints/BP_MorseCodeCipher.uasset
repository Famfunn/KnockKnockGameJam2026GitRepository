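; BP_MorseCodeCipher is an interactable object that brings up the Morse code cipher UI.
; Interact fires CodeCipherAppearEvent and returns the static mesh of ObjectMesh to the caller.
; The event creates a new WBP_MorseCodeCipher widget, adds it to the viewport, switches player 0 to UI-only input and shows the mouse cursor.
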(event Custom|CodeCipherAppearEvent
  (bind _returnvalue (Game|GetPlayerController 0))
  (bind _returnvalue_2 (UserInterface|CreateWidget "/Game/UI/WBP_MorseCodeCipher.WBP_MorseCodeCipher_C"))
  (UserInterface|Viewport|AddtoViewport _returnvalue_2 0)
  (Input|SetInputModeUIOnly _returnvalue 0 "DoNotLock" true)
  (Variables|/Script/Engine.PlayerController|SetbShowMouseCursor _returnvalue true))

(fn ConstructionScript
  (|CallParentFunction))

(fn Interact
  (CallFunction|CodeCipherAppearEvent)
  (return (Variables|/Script/Engine.StaticMeshComponent|GetStaticMesh (Variables|Default|GetObject%20Mesh))))