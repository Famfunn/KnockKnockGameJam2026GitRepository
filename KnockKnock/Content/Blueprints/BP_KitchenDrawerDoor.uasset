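; Kitchen drawer door Blueprint that swings open when interacted with and closes itself a few seconds later.
; Interact calls Drawer2Open and returns the Drawer2 static mesh to the caller.
; Drawer2Open snaps Drawer2 90 degrees in local pitch without animation, then reverses it after a delay.
; A DoOnce blocks retriggering until the door has closed and the gate resets.
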(event Custom|Drawer2Open
  (Utilities|FlowControl|DoOnce false :!label _label
    (:Completed
      (Transformation|AddLocalRotation (Variables|Default|GetDrawer2) (Math|Rotator|MakeRotator 0.0 9e+01 0.0) false false)
      (Utilities|FlowControl|Delay 5.0)
      (Transformation|AddLocalRotation (Variables|Default|GetDrawer2) "-90.000000,0.000000,0.000000" false false)
      (goto _label Reset))))

(fn ConstructionScript)

(fn Interact
  (CallFunction|Drawer2Open)
  (return (Variables|/Script/Engine.StaticMeshComponent|GetStaticMesh (Variables|Default|GetDrawer2))))