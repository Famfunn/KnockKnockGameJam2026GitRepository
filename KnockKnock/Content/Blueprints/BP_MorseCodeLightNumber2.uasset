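; Morse code light actor that repeatedly flashes the digit 5 as short dots, despite the Number2 in its name.
; BeginPlay chains point light visibility toggles with short equal delays, prints "5" as a debug string, pauses, then loops back to the start.
; The timing is hardcoded node by node rather than data-driven.
; An Interact function returns the light mesh's static mesh.
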(event EventBeginPlay
  ;[1 1 1] This is a dash in morse code (in terms of flashing the light), 0.5 sec per flash for dash, 0.2 sec per flash for dot (will play around with these values)
  (Utilities|FlowControl|RetriggerableDelay 1.0 :!label _label)
  (Rendering|ToggleVisibility (Variables|Default|GetPointLight) false)
  (Utilities|FlowControl|Delay 0.2)
  ;[1 1 1] Code for Number 5
  (Rendering|ToggleVisibility (Variables|Default|GetPointLight) false)
  (Utilities|FlowControl|Delay 0.2)
  (Rendering|ToggleVisibility (Variables|Default|GetPointLight) false)
  (Utilities|FlowControl|Delay 0.2)
  (Rendering|ToggleVisibility (Variables|Default|GetPointLight) false)
  (Utilities|FlowControl|Delay 0.2)
  (Rendering|ToggleVisibility (Variables|Default|GetPointLight) false)
  (Utilities|FlowControl|Delay 0.2)
  (Rendering|ToggleVisibility (Variables|Default|GetPointLight) false)
  (Utilities|FlowControl|Delay 0.2)
  (Rendering|ToggleVisibility (Variables|Default|GetPointLight) false)
  (Utilities|FlowControl|Delay 0.2)
  (Rendering|ToggleVisibility (Variables|Default|GetPointLight) false)
  (Utilities|FlowControl|Delay 0.2)
  (Rendering|ToggleVisibility (Variables|Default|GetPointLight) false)
  (Utilities|FlowControl|Delay 0.2)
  (Rendering|ToggleVisibility (Variables|Default|GetPointLight) false)
  (Utilities|FlowControl|Delay 0.2)
  (Rendering|ToggleVisibility (Variables|Default|GetPointLight) false)
  (Development|PrintString "5")
  (Rendering|ToggleVisibility (Variables|Default|GetPointLight) false)
  (Utilities|FlowControl|RetriggerableDelay 3.0)
  (for _index (range 0 0)
    _)
  (goto _label))

(fn ConstructionScript)

(fn Interact
  (return (Variables|/Script/Engine.StaticMeshComponent|GetStaticMesh (Variables|Default|GetLightMesh))))